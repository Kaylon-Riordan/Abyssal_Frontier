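; BP_LightManager is a Blueprint that sets the brightness of powered lights in the level according to a stepped Power level.
; SetLights looks up the intensity for the current Power, applies it to every Light tagged "Powered Light", and writes it to the MPC_Lights emissive strength parameter.
; Init applies the current level, while IncreasePower raises it by one without a bounds check and reapplies it.
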(event Custom|Increase%20Power
  (Math|Integer|IncrementInt (Variables|Default|GetPower)
    (:%20%20
      (CallFunction|SetLights))))

(event Custom|Set%20Lights
  (bind _light_intensities (Variables|Default|GetLight%20Intensities))
  (bind _power (Variables|Default|GetPower))
  (bind _output (Utilities|Array|Get(acopy) _light_intensities _power))
  (bind _outactors (Actor|GetAllActorswithTag "Powered Light"))
  (for _array_element _outactors
    (bind _aslight (Utilities|Casting|CastToLight _array_element))
    (Rendering|Components|Light|SetIntensity (Variables|/Script/Engine.Light|GetLightComponent _aslight) _output))
  (Rendering|Material|SetScalarParameterValue "/Game/Materials/MPC_Lights.MPC_Lights" "Emmisive Strenght" _output :!class /Script/Engine.KismetMaterialLibrary)
  (Development|PrintString (Utilities|String|ToString(Integer) _power)))

(event EventInit
  (CallFunction|SetLights))