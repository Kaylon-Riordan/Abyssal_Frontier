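; BP_PowerSlot is a power slot that takes a battery once and raises the power tracked by the light manager.
; On Activate, an empty slot casts the game instance to BP_LightManager and calls IncreasePower.
; It then reveals the Cylinder03 component, marks itself Full so later activations do nothing, and plays a battery slot-in sound at the world origin.
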(event EventActivate
  (if (not (Variables|Default|GetFull))
    (bind _asbp_light_manager (Utilities|Casting|CastToBP_LightManager (Game|GetGameInstance)))
    (Default|IncreasePower _asbp_light_manager)
    (Rendering|SetVisibility (Variables|Default|Getcylinder_03) true false)
    (Variables|Default|SetFull true)
    (Audio|PlaySoundatLocation "/Game/Audio/Sounds/SFX_Battery_SlotIn_01.SFX_Battery_SlotIn_01" "0, 0, 0" "0, 0, 0" 1.0 1.0 0.0 0 0 0 0)))

(fn ConstructionScript
  (|CallParentFunction))