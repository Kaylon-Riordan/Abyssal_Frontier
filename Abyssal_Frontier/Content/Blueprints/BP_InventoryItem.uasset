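; BP_InventoryItem is an interactable pickup actor that hands itself to the player character's inventory.
; Its construction script sets the interactable mesh from the mesh in its Item data.
; On InteractEvent it plays a hardcoded battery pickup sound at its location, then casts to BP_HorrorCharacter and calls InventoryInteract on that character's inventory component with itself as the argument.
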(event EventBeginPlay
  (|CallParentFunction) ; This node is disabled and will not be called.\nDrag off pins to build functionality.
)

(event Collision|EventActorBeginOverlap
  (params (OtherActor :type Actor%20Object%20Reference))
  (|CallParentFunction OtherActor) ; This node is disabled and will not be called.\nDrag off pins to build functionality.
)

(event EventTick
  (params (DeltaSeconds :type Float%20%28single-precision%29))
  (|CallParentFunction DeltaSeconds) ; This node is disabled and will not be called.\nDrag off pins to build functionality.
)

(event EventInteractEvent
  (params (Character :type Actor%20Object%20Reference))
  (Audio|PlaySoundatLocation "/Game/Audio/Sounds/SFX_Battery_PickUp_01.SFX_Battery_PickUp_01" (Transformation|GetActorLocation) "0, 0, 0" 1.0 1.0 0.0 0 0 0 0)
  (bind _asbp_horror_character (Utilities|Casting|CastToBP_HorrorCharacter Character))
  (bind _asbp_inventory_component (Utilities|Casting|CastToBP_InventoryComponent (Variables|/Game/Blueprints/BP_HorrorCharacter.BP_HorrorCharacter_C|GetBP_InventoryComponent _asbp_horror_character)))
  (Default|InventoryInteract _asbp_inventory_component self))

(fn ConstructionScript
  (|CallParentFunction)
  (Components|StaticMesh|SetStaticMesh (Variables|Default|GetInteractable%20Mesh) (.Mesh (Utilities|Struct|BreakS_ItemStructure (Variables|Default|GetItem)))))