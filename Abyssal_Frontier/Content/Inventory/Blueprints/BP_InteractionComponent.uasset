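; Interaction component that lets the player hover and use BP_InteractableBase actors at screen center by pressing E.
; Overlap events keep a count that runs a looping sight-check timer only while interactables are in range.
; Each check sphere-traces from the deprojected viewport center, with debug drawing on, for actors tagged Interactable.
; The hit sets the current object and drives hover callbacks; E passes the owner to its InteractEvent.
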(event Custom|On%20Interactable%20Overlap
  (params (Overlap :type Boolean))
  (Utilities|FlowControl|Sequence
    (:then_0
      (Variables|Default|SetOverlap%20Count (+ (Variables|Default|GetOverlap%20Count) (select Overlap 1 -1))))
    (:then_1
      (CallFunction|DrawTrace (> (Variables|Default|GetOverlap%20Count) 0)))))

(event Custom|Draw%20Trace
  (params (Draw%20Trace :type Boolean))
  (if Draw%20Trace
    (if (not (Utilities|Time|IsValidTimerHandle (Variables|Default|GetTrace%20Timer)))
      (bind _returnvalue (Utilities|Time|SetTimerbyFunctionName 0 "Detect Sight" 0.1 true))
      (Variables|Default|SetTrace%20Timer _returnvalue))
    (elif (Utilities|Time|IsValidTimerHandle (Variables|Default|GetTrace%20Timer))
      (Utilities|Time|ClearandInvalidateTimerbyHandle (Variables|Default|GetTrace%20Timer))
      (bind _interactable_object (Variables|Default|GetInteractable%20Object)
        (:then
          (bind _asbp_interactable_base (Utilities|Casting|CastToBP_InteractableBase _interactable_object))
          (Default|OnUnhover _asbp_interactable_base)
          (Variables|Default|SetInteractable%20Object 0)
          (Variables|Default|SetCan%20Interact false))
        (:else)))))

(event Custom|Detect%20Sight
  (bind _returnvalue (Game|GetPlayerController 0))
  (bind (_sizex _sizey) (HUD|GetViewportSize _returnvalue))
  (bind _returnvalue_2 (/ _sizey 2))
  (bind _returnvalue_3 (/ _sizex 2))
  (bind _returnvalue_4 (Math|Conversions|ToFloat(Integer) _returnvalue_3))
  (bind _returnvalue_5 (Math|Conversions|ToFloat(Integer) _returnvalue_2))
  (bind (_worldlocation _worlddirection) (Class|PlayerController|DeprojectScreenPositiontoWorld _returnvalue _returnvalue_4 _returnvalue_5))
  (bind (_outhit _returnvalue_6) (Collision|SphereTraceByChannel _worldlocation (+ _worldlocation (* _worlddirection 2.5e+02)) 5.0 "TraceTypeQuery1" false 0 "ForDuration" true "(R=1.000000,G=0.000000,B=0.000000,A=1.000000)" "(R=0.000000,G=1.000000,B=0.000000,A=1.000000)" 0.1))
  (if _returnvalue_6
    (if (Actor|ActorHasTag (.HitActor (Collision|BreakHitResult _outhit)) "Interactable")
      (if (not (== (.HitActor (Collision|BreakHitResult _outhit)) (Variables|Default|GetInteractable%20Object)))
        (bind _asbp_interactable_base (Utilities|Casting|CastToBP_InteractableBase (.HitActor (Collision|BreakHitResult _outhit))))
        (Default|OnUnhover _asbp_interactable_base)
        (bind _output_get (Variables|Default|SetInteractable%20Object (.HitActor (Collision|BreakHitResult _outhit))))
        (Variables|Default|SetCan%20Interact true)
        (bind _asbp_interactable_base_2 (Utilities|Casting|CastToBP_InteractableBase _output_get))
        (Default|OnHover _asbp_interactable_base_2))
      (else
        (bind _interactable_object (Variables|Default|GetInteractable%20Object :!label _label)
          (:then
            (bind _asbp_interactable_base_3 (Utilities|Casting|CastToBP_InteractableBase _interactable_object))
            (Default|OnUnhover _asbp_interactable_base_3)
            (Variables|Default|SetInteractable%20Object 0)
            (Variables|Default|SetCan%20Interact false))
          (:else))))
    (else
      (goto _label))))

(event Input|KeyboardEvents|E
  (params (Key :type Key%20Structure :default "None"))
  (:Pressed
    (if (Variables|Default|GetCan%20Interact)
      (bind _asbp_interactable_base (Utilities|Casting|CastToBP_InteractableBase (Variables|Default|GetInteractable%20Object)))
      (Default|InteractEvent _asbp_interactable_base (Components|GetOwner)))))