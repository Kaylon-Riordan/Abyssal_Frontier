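; Base interactable actor for the inventory system that the player can hover over and interact with.
; Its collision sphere notifies the player character's BP_InteractionComponent when the player enters or leaves range.
; Hover events toggle custom depth rendering on InteractableMesh and print debug text.
; InteractEvent takes a character and only prints a placeholder message.
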(event OnComponentBeginOverlap(CollisionSphere)
  (params (OverlappedComponent :type Primitive%20Component%20Object%20Reference) (OtherActor :type Actor%20Object%20Reference) (OtherComp :type Primitive%20Component%20Object%20Reference) (OtherBodyIndex :type Integer) (bFromSweep :type Boolean) (SweepResult :type Hit%20Result%20Structure%20%28by%20ref%29))
  (bind _returnvalue (Actor|GetComponentbyClass OtherActor "/Game/Inventory/Blueprints/BP_InteractionComponent.BP_InteractionComponent_C"))
  (if (== OtherActor (Game|GetPlayerCharacter 0))
    (if (Utilities|IsValid _returnvalue)
      (Default|OnInteractableOverlap _returnvalue true))))

(event OnComponentEndOverlap(CollisionSphere)
  (params (OverlappedComponent :type Primitive%20Component%20Object%20Reference) (OtherActor :type Actor%20Object%20Reference) (OtherComp :type Primitive%20Component%20Object%20Reference) (OtherBodyIndex :type Integer))
  (bind _returnvalue (Actor|GetComponentbyClass OtherActor "/Game/Inventory/Blueprints/BP_InteractionComponent.BP_InteractionComponent_C"))
  (if (== OtherActor (Game|GetPlayerCharacter 0))
    (if (Utilities|IsValid _returnvalue)
      (Default|OnInteractableOverlap _returnvalue false))))

(event Custom|On%20Hover
  (Rendering|SetRenderCustomDepth (Variables|Default|GetInteractable%20Mesh) true)
  (Development|PrintString "Hello"))

(event Custom|On%20Unhover
  (Rendering|SetRenderCustomDepth (Variables|Default|GetInteractable%20Mesh) false)
  (Development|PrintString "Goodbye"))

(event Custom|Interact%20Event
  (params (Character :type Actor%20Object%20Reference))
  (Development|PrintString "Interact"))

(event EventBeginPlay)

(event Collision|EventActorBeginOverlap
  (params (OtherActor :type Actor%20Object%20Reference)))

(event EventTick
  (params (DeltaSeconds :type Float%20%28single-precision%29)))

(fn ConstructionScript)